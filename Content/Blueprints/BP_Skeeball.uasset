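; BP_Skeeball is a skeeball machine that starts a game when a BP_MotionController fingertip overlaps its PlayBoxDetector.
; BeginGame resets score and balls, plays music and spawns four staggered BP_PickupBall actors.
; Hole triggers use up a ball, add points and spawn replacements while more than three remain; only the zero-point trigger destroys the overlapping actor.
; At zero balls it shows game over and records the high score.
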(event OnComponentBeginOverlap(ZeroPts)
  (params (OverlappedComponent :type Primitive%20Component%20Object%20Reference) (OtherActor :type Actor%20Object%20Reference) (OtherComp :type Primitive%20Component%20Object%20Reference) (OtherBodyIndex :type Integer) (bFromSweep :type Boolean) (SweepResult :type Hit%20Result%20Structure%20%28by%20ref%29))
  (Variables|Default|SetBallsRemaining (- (Variables|Default|GetBallsRemaining) 1))
  (Audio|Components|Audio|Play (Variables|Default|GetBallHole) 0.0)
  (CallFunction|SpawnNewBall)
  (Actor|DestroyActor OtherActor)
  (CallFunction|UpdateScore)
  (CallFunction|IsGameOver)
  (CallFunction|UpdateScore))

(event OnComponentBeginOverlap(50PtsTrigger)
  (params (OverlappedComponent :type Primitive%20Component%20Object%20Reference) (OtherActor :type Actor%20Object%20Reference) (OtherComp :type Primitive%20Component%20Object%20Reference) (OtherBodyIndex :type Integer) (bFromSweep :type Boolean) (SweepResult :type Hit%20Result%20Structure%20%28by%20ref%29))
  (Variables|Default|SetBallsRemaining (- (Variables|Default|GetBallsRemaining) 1))
  (Audio|Components|Audio|Play (Variables|Default|GetBallHole) 0.0)
  (CallFunction|SpawnNewBall)
  (Variables|Default|SetScore (+ (Variables|Default|GetScore) 50))
  (CallFunction|UpdateScore)
  (CallFunction|IsGameOver)
  (CallFunction|UpdateScore))

(event OnComponentBeginOverlap(40PtsTrigger)
  (params (OverlappedComponent :type Primitive%20Component%20Object%20Reference) (OtherActor :type Actor%20Object%20Reference) (OtherComp :type Primitive%20Component%20Object%20Reference) (OtherBodyIndex :type Integer) (bFromSweep :type Boolean) (SweepResult :type Hit%20Result%20Structure%20%28by%20ref%29))
  (Variables|Default|SetBallsRemaining (- (Variables|Default|GetBallsRemaining) 1))
  (Audio|Components|Audio|Play (Variables|Default|GetBallHole) 0.0)
  (CallFunction|SpawnNewBall)
  (Variables|Default|SetScore (+ (Variables|Default|GetScore) 40))
  (CallFunction|UpdateScore)
  (CallFunction|IsGameOver)
  (CallFunction|UpdateScore))

(event OnComponentBeginOverlap(100PtsTriggerLeft)
  (params (OverlappedComponent :type Primitive%20Component%20Object%20Reference) (OtherActor :type Actor%20Object%20Reference) (OtherComp :type Primitive%20Component%20Object%20Reference) (OtherBodyIndex :type Integer) (bFromSweep :type Boolean) (SweepResult :type Hit%20Result%20Structure%20%28by%20ref%29))
  (Variables|Default|SetBallsRemaining (- (Variables|Default|GetBallsRemaining) 1))
  (Audio|Components|Audio|Play (Variables|Default|GetBallHole) 0.0)
  (CallFunction|SpawnNewBall)
  (Variables|Default|SetScore (+ (Variables|Default|GetScore) 100))
  (CallFunction|UpdateScore)
  (CallFunction|IsGameOver)
  (CallFunction|UpdateScore))

(event OnComponentBeginOverlap(100PtsTriggerRight)
  (params (OverlappedComponent :type Primitive%20Component%20Object%20Reference) (OtherActor :type Actor%20Object%20Reference) (OtherComp :type Primitive%20Component%20Object%20Reference) (OtherBodyIndex :type Integer) (bFromSweep :type Boolean) (SweepResult :type Hit%20Result%20Structure%20%28by%20ref%29))
  (Variables|Default|SetBallsRemaining (- (Variables|Default|GetBallsRemaining) 1))
  (Audio|Components|Audio|Play (Variables|Default|GetBallHole) 0.0)
  (CallFunction|SpawnNewBall)
  (Variables|Default|SetScore (+ (Variables|Default|GetScore) 100))
  (CallFunction|UpdateScore)
  (CallFunction|IsGameOver)
  (CallFunction|UpdateScore))

(event OnComponentBeginOverlap(10PtsTrigger)
  (params (OverlappedComponent :type Primitive%20Component%20Object%20Reference) (OtherActor :type Actor%20Object%20Reference) (OtherComp :type Primitive%20Component%20Object%20Reference) (OtherBodyIndex :type Integer) (bFromSweep :type Boolean) (SweepResult :type Hit%20Result%20Structure%20%28by%20ref%29))
  (Variables|Default|SetBallsRemaining (- (Variables|Default|GetBallsRemaining) 1))
  (Audio|Components|Audio|Play (Variables|Default|GetBallHole) 0.0)
  (CallFunction|SpawnNewBall)
  (Variables|Default|SetScore (+ (Variables|Default|GetScore) 10))
  (CallFunction|UpdateScore)
  (CallFunction|IsGameOver)
  (CallFunction|UpdateScore))

(event OnComponentBeginOverlap(30PtsTrigger)
  (params (OverlappedComponent :type Primitive%20Component%20Object%20Reference) (OtherActor :type Actor%20Object%20Reference) (OtherComp :type Primitive%20Component%20Object%20Reference) (OtherBodyIndex :type Integer) (bFromSweep :type Boolean) (SweepResult :type Hit%20Result%20Structure%20%28by%20ref%29))
  (Variables|Default|SetBallsRemaining (- (Variables|Default|GetBallsRemaining) 1))
  (Audio|Components|Audio|Play (Variables|Default|GetBallHole) 0.0)
  (CallFunction|SpawnNewBall)
  (Variables|Default|SetScore (+ (Variables|Default|GetScore) 30))
  (CallFunction|UpdateScore)
  (CallFunction|IsGameOver)
  (CallFunction|UpdateScore))

(event OnComponentBeginOverlap(20PtsTrigger)
  (params (OverlappedComponent :type Primitive%20Component%20Object%20Reference) (OtherActor :type Actor%20Object%20Reference) (OtherComp :type Primitive%20Component%20Object%20Reference) (OtherBodyIndex :type Integer) (bFromSweep :type Boolean) (SweepResult :type Hit%20Result%20Structure%20%28by%20ref%29))
  (Variables|Default|SetBallsRemaining (- (Variables|Default|GetBallsRemaining) 1))
  (Audio|Components|Audio|Play (Variables|Default|GetBallHole) 0.0)
  (CallFunction|SpawnNewBall)
  (Variables|Default|SetScore (+ (Variables|Default|GetScore) 20))
  (CallFunction|UpdateScore)
  (CallFunction|IsGameOver)
  (CallFunction|UpdateScore))

(event OnComponentBeginOverlap(PlayBoxDetector)
  (params (OverlappedComponent :type Primitive%20Component%20Object%20Reference) (OtherActor :type Actor%20Object%20Reference) (OtherComp :type Primitive%20Component%20Object%20Reference) (OtherBodyIndex :type Integer) (bFromSweep :type Boolean) (SweepResult :type Hit%20Result%20Structure%20%28by%20ref%29))
  (bind _asbp_motion_controller (Utilities|Casting|CastToBP_MotionController OtherActor))
  (if (== OtherComp (Variables|/Game/Blueprints/BP_MotionController.BP_MotionController_C|GetFingerTip _asbp_motion_controller))
    (if (not (Variables|Default|GetIsGamePlaying))
      (CallFunction|BeginGame))))

(event Custom|SpawnInitialBalls
  (Audio|Components|Audio|Play (Variables|Default|GetBallSpawn) 0.0)
  (CallFunction|SpawnNewBall)
  (Utilities|FlowControl|Delay 0.5)
  (CallFunction|SpawnNewBall)
  (Utilities|FlowControl|Delay 0.5)
  (CallFunction|SpawnNewBall)
  (Utilities|FlowControl|Delay 0.5)
  (CallFunction|SpawnNewBall))

(event Custom|BeginGame
  (Variables|Default|SetIsGamePlaying true)
  (Rendering|SetVisibility (Variables|Default|GetGameOverText) false false)
  (Variables|Default|SetBallsRemaining (Variables|Default|GetMaxBalls))
  (Variables|Default|SetScore 0)
  (CallFunction|UpdateScore)
  (CallFunction|SpawnInitialBalls)
  (Audio|Components|Audio|Play (Variables|Default|GetMusic) 0.0))

(event EventTick
  (params (DeltaSeconds :type Float%20%28single-precision%29))
  (Rendering|Debug|FlushPersistentDebugLines)
  (Development|PrintString (Utilities|String|ToString(Integer) (Variables|Default|GetBallsRemaining)) true false))

(fn ConstructionScript)

(fn SpawnNewBall
  (if (> (Variables|Default|GetBallsRemaining) 3)
    (Game|SpawnActorfromClass "/Game/Blueprints/BP_PickupBall.BP_PickupBall_C" (Math|Transform|MakeTransform (Transformation|GetWorldLocation (Variables|Default|GetBallSpawnLocation)) "0, 0, 0" "1,1,1") "Undefined" 0 0)))

(fn UpdateScore
  (Rendering|Components|TextRender|SetText (Variables|Default|GetScoreText) (Utilities|Text|ToText(Integer) (Variables|Default|GetScore)))
  (Rendering|Components|TextRender|SetText (Variables|Default|GetHighScoreText) (Utilities|Text|ToText(String) (Utilities|String|Append "High Score: " (Utilities|String|ToString(Integer) (Variables|Default|GetHighScore))))))

(fn IsGameOver
  (if (== (Variables|Default|GetBallsRemaining) 0)
    (Variables|Default|SetIsGamePlaying false)
    (Rendering|SetVisibility (Variables|Default|GetGameOverText) true false)
    (if (> (Variables|Default|GetScore) (Variables|Default|GetHighScore))
      (Variables|Default|SetHighScore (Variables|Default|GetScore)))))